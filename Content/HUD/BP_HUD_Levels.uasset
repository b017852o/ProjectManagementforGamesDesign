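; BP_HUD_Levels is a level HUD Blueprint that shows a running timer on screen.
; On BeginPlay it creates a WBP_Timer widget for the first player, adds it to the viewport and starts the count from zero.
; A looping one-millisecond timer event increments Time by a fixed step and pushes it to the widget, counting timer firings rather than reading the game clock.
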(event Custom|StartTimer
  (Variables|Default|SetTime 0.0)
  (bind _returnvalue (Utilities|Time|SetTimerbyEvent (delegate Custom|100thMillisecond) 0.001 true))
  (Variables|Default|SetTimer _returnvalue)
  (Default|SetTime (Variables|Default|GetHUDTimer) (stale Custom|100thMillisecond _output_get)))

(event Custom|100thMillisecond
  (bind _output_get (Variables|Default|SetTime (+ (Variables|Default|GetTime) 0.001)))
  (Default|SetTime (Variables|Default|GetHUDTimer) _output_get))

(event EventBeginPlay
  (bind _returnvalue (UserInterface|CreateWidget "/Game/WidgetUI/WBP_Timer.WBP_Timer_C" (Game|GetPlayerController 0)))
  (bind _output_get (Variables|Default|SetHUDTimer _returnvalue))
  (UserInterface|Viewport|AddtoViewport _output_get 0)
  (CallFunction|StartTimer))

(fn ConstructionScript)